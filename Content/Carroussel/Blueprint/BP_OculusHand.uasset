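; Oculus hand-tracking component that detects grab and pinch gestures for either hand and fires grab, pinch and release events on state changes.
; After a startup delay it waits for high tracking confidence, with a single timed retry, then caches fingertip bones and enables tick.
; Each tick, average fingertip-to-wrist distance maps to a grab axis compared against a threshold.
; Pinch compares index-to-thumb pad distance against a limit.
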(event Custom|CustomEvent
  (if (Utilities|Enum|Equal(Enum) (Class|OculusXRInputFunctionLibrary|GetTrackingConfidence (Variables|Default|GetMeshType)) "High")
    (Utilities|Time|ClearandInvalidateTimerbyHandle (stale EventBeginPlay _returnvalue))
    (for _index (range 0 (- (Class|SkinnedMeshComponent|GetNumBones) 1))
      (if (Utilities|String|Contains (Utilities|String|ToLower (Utilities|String|ToString(Name) (Class|SkinnedMeshComponent|GetBoneName _index))) "tip")
        (Utilities|Array|Add (Variables|Z-Settings|GetFingerTips) (Class|SkinnedMeshComponent|GetBoneName _index))))
    (Components|Tick|SetComponentTickEnabled true)
    (Development|PrintString "isEnabled")))

(event EventBeginPlay
  (Utilities|FlowControl|Delay 1.0)
  (if (Utilities|Enum|Equal(Enum) (Class|OculusXRInputFunctionLibrary|GetTrackingConfidence (Variables|Default|GetMeshType)) "High")
    (for _index (range 0 (- (Class|SkinnedMeshComponent|GetNumBones) 1))
      (if (Utilities|String|Contains (Utilities|String|ToLower (Utilities|String|ToString(Name) (Class|SkinnedMeshComponent|GetBoneName _index))) "tip")
        (Utilities|Array|Add (Variables|Z-Settings|GetFingerTips) (Class|SkinnedMeshComponent|GetBoneName _index))))
    (Components|Tick|SetComponentTickEnabled true)
    (Development|PrintString "isEnabled")
    (else
      (bind _returnvalue (Utilities|Time|SetTimerbyEvent (delegate Custom|CustomEvent) 0.1)))))

(event EventTick
  (params (DeltaSeconds :type Float%20%28single-precision%29))
  (Utilities|FlowControl|Sequence
    (:then_0
      (if (CallFunction|DetectGrabbing)
        (if (not (Variables|Z-Settings|GetbGrabbed))
          (Default|CallOnHandGrab)
          (Variables|Z-Settings|SetbGrabbed true))
        (elif (Variables|Z-Settings|GetbGrabbed)
          (Default|CallOnHandRelease)
          (Variables|Z-Settings|SetbGrabbed false))))
    (:then_1
      (if (CallFunction|DetectPinching)
        (if (not (Variables|Z-Settings|GetbPinched))
          (Default|CallOnHandPinch)
          (Variables|Z-Settings|SetbPinched true)
          (Development|PrintString "Pinched"))
        (elif (Variables|Z-Settings|GetbPinched)
          (Default|CallOnHandPinchRelease)
          (Variables|Z-Settings|SetbPinched false)
          (Development|PrintString "Unpinched"))))))

(fn DetectGrabbing
  (for _array_element (Variables|Z-Settings|GetFingerTips)
    (bind _returnvalue (Class|PoseableMeshComponent|GetBoneLocationbyName _array_element "WorldSpace"))
    (bind _returnvalue_2 (Class|PoseableMeshComponent|GetBoneLocationbyName (Utilities|Select :Index (Variables|Default|GetMeshType) :None "None" :HandLeft "b_l_wrist" :HandRight "b_r_wrist") "WorldSpace"))
    (Utilities|Array|Add (LocalVariables|GetDIstances) (Math|Float|Absolute(Float) (Math|Vector|VectorLength (- _returnvalue_2 _returnvalue)))))
  (for _array_element_2 (LocalVariables|GetDIstances)
    (LocalVariables|SetTotalDistance (+ _array_element_2 (LocalVariables|GetTotalDistance))))
  (if (== (LocalVariables|GetTotalDistance) 0.0)
    (return false)
    (else
      (bind _output_get (LocalVariables|SetDistanceAverage (/ (LocalVariables|GetTotalDistance) (Utilities|Array|Length (LocalVariables|GetDIstances)))))
      (bind _output_get_2 (Variables|Z-Settings|SetGrabAxis (Math|Float|MapRangeClamped _output_get 7.8 16.9 1.0 0.0)))
      (if (> _output_get_2 (Variables|GrabSettings|GetGrabThreshold))
        (return true)
        (else
          (return false))))))

(fn DetectPinching
  (Utilities|FlowControl|Sequence
    (:then_0
      (bind _returnvalue (Class|PoseableMeshComponent|GetBoneLocationbyName (Utilities|Select :Index (Variables|Default|GetMeshType) :None "None" :HandLeft "l_index_finger_pad_marker" :HandRight "r_index_finger_pad_marker") "WorldSpace"))
      (bind _returnvalue_2 (Class|PoseableMeshComponent|GetBoneLocationbyName (Utilities|Select :Index (Variables|Default|GetMeshType) :None "None" :HandLeft "l_thumb_finger_pad_marker" :HandRight "r_thumb_finger_pad_marker") "WorldSpace"))
      (LocalVariables|SetFingerDistance (Math|Float|Absolute(Float) (Math|Vector|VectorLength (- _returnvalue_2 _returnvalue)))))
    (:then_1
      (return (< (LocalVariables|GetFingerDistance) (Variables|Z-Settings|GetPinchAxis))))))