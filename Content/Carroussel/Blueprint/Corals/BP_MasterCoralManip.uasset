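; Master coral actor for the carousel, which can be grabbed by a hand, scaled, and shown in low or high detail.
; A bubble HandDetector forwards overlaps to the carousel; other events swap meshes and opaque or translucent materials.
; Zoom adds an offset to the high-def mesh's captured scale, applying only results above 1.
; Selection toggles Tick, which interpolates opacity but writes it to parameter "None"; Release is empty.
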(event OnComponentBeginOverlap(HandDetector)
  (params (OverlappedComponent :type Primitive%20Component%20Object%20Reference) (OtherActor :type Actor%20Object%20Reference) (OtherComp :type Primitive%20Component%20Object%20Reference) (OtherBodyIndex :type Integer) (bFromSweep :type Boolean) (SweepResult :type Hit%20Result%20Structure%20%28by%20ref%29))
  (Default|HandBeginOverlap (Variables|Default|GetCarrouselRef) OtherComp))

(event OnComponentEndOverlap(HandDetector)
  (params (OverlappedComponent :type Primitive%20Component%20Object%20Reference) (OtherActor :type Actor%20Object%20Reference) (OtherComp :type Primitive%20Component%20Object%20Reference) (OtherBodyIndex :type Integer))
  (Default|HandEndOverlap (Variables|Default|GetCarrouselRef) OtherComp))

(event Custom|SwitchToOpaque
  (Rendering|Material|SetMaterial (Variables|Default|GetHighDefMesh) 0 "/Game/Carroussel/Materials/Mat_CoralOpdaque.Mat_CoralOpdaque"))

(event Custom|SwitchToTransparent
  (Rendering|Material|SetMaterial (Variables|Default|GetHighDefMesh) 0 "/Game/Carroussel/Materials/Mat_CoralTranslucent.Mat_CoralTranslucent"))

(event Custom|UpdateScale
  (params (NewScaleOffset :type Float%20%28double-precision%29))
  (if (Variables|Default|GetbIsZooming)
    (if (> (+ NewScaleOffset (Variables|Default|GetInitialScale)) 1.0)
      (Variables|Default|SetActualScale (+ NewScaleOffset (Variables|Default|GetInitialScale)))
      (Transformation|SetWorldScale3D (Variables|Default|GetHighDefMesh) (Math|Conversions|ToVector(Float) (+ NewScaleOffset (Variables|Default|GetInitialScale)))))
    (else
      (Variables|Default|SetbIsZooming true)
      (Variables|Default|SetInitialScale (.x (Transformation|GetWorldScale (Variables|Default|GetHighDefMesh)))))))

(event Custom|ResetScale
  (Variables|Default|SetbIsZooming false))

(event Custom|SwitchToLowDefCoral
  (CallFunction|ShowCoral)
  (if (Variables|Default|GetbIsHighDef)
    (Development|SetHiddeninGame (Variables|Default|GetHighDefMesh) true false)))

(event Custom|DeselectCoral
  (Actor|Tick|SetActorTickEnabled false))

(event Custom|SelectCoral
  (Actor|Tick|SetActorTickEnabled true))

(event Custom|SwitchToHighDefCoral
  (Variables|Default|SetbIsHighDef true)
  (CallFunction|HideCoral)
  (Development|SetHiddeninGame (Variables|Default|GetHighDefMesh) false false))

(event Custom|Grab
  (params (HandToAttach :type Scene%20Component%20Object%20Reference))
  (Transformation|AttachComponentToComponent HandToAttach "None" "KeepRelative" "KeepRelative" "KeepRelative" true))

(event Custom|ShowCoral
  (Development|SetHiddeninGame (Variables|Default|GetHandDetector) false false))

(event Custom|HideCoral
  (Development|SetHiddeninGame (Variables|Debug|GetStaticMeshComponent) true false))

(event Custom|Release)

(event EventBeginPlay
  (bind _highdefmesh (Variables|Default|GetHighDefMesh))
  (Utilities|IsValid (Variables|/Script/Engine.StaticMeshComponent|GetStaticMesh (Variables|Default|GetHighDefMesh))
    (:Is%20Not%20Valid
      (Components|StaticMesh|SetStaticMesh _highdefmesh (Variables|/Script/Engine.StaticMeshComponent|GetStaticMesh (Variables|Debug|GetStaticMeshComponent)))
      (Rendering|Material|SetMaterial _highdefmesh 0 "/Game/Carroussel/Materials/Mat_CoralOpdaque.Mat_CoralOpdaque"))))

(event Collision|EventActorBeginOverlap
  (params (OtherActor :type Actor%20Object%20Reference)))

(event EventTick
  (params (DeltaSeconds :type Float%20%28single-precision%29))
  (bind _output_get (Variables|Default|SetActualOpacityLevel (Math|Interpolation|FInterptoConstant (Variables|Default|GetActualOpacityLevel) (Variables|Default|GetOpacityWanted) DeltaSeconds 6.0)))
  (Rendering|Material|SetScalarParameterValueonMaterials (Variables|Debug|GetStaticMeshComponent) "None" _output_get))

(fn ConstructionScript
  (Rendering|Material|SetMaterial (Variables|Debug|GetStaticMeshComponent) 0 "/Game/Carroussel/Materials/Mat_CoralOpdaque.Mat_CoralOpdaque")
  (Rendering|Material|SetMaterial (Variables|Default|GetHandDetector) 0 "/Game/Carroussel/Materials/MatI_CarrouselBubble_Inst.MatI_CarrouselBubble_Inst")
  (bind _highdefmesh (Variables|Default|GetHighDefMesh)
    (:then
      (Rendering|Material|SetMaterial _highdefmesh 0 "/Game/Carroussel/Materials/Mat_CoralOpdaque.Mat_CoralOpdaque"))
    (:else)))