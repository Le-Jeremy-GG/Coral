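; Tracked VR hand Blueprint for the Carroussel content, wrapping a motion controller and an Oculus hand for the side chosen by its Hand enum.
; The construction script applies that enum to the controller's motion source and to the hand's mesh and skeleton types, so one Blueprint can serve either hand.
; Grab and release events from the hand only print the hand name and action.
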(event OnHandGrab(BP_OculusHand)
  (Development|PrintString (Utilities|String|Append (Utilities|String|EnumtoString (Variables|Default|GetHand)) "Grab")))

(event OnHandRelease(BP_OculusHand)
  (Development|PrintString (Utilities|String|Append (Utilities|String|EnumtoString (Variables|Default|GetHand)) "Release")))

(fn ConstructionScript
  (bind _bp_oculushand (Variables|Default|GetBP_OculusHand))
  (Variables|/Script/HeadMountedDisplay.MotionControllerComponent|SetMotionSource (Variables|Default|GetMotionController) (Utilities|Name|EnumtoName (Variables|Default|GetHand)))
  (Variables|/Script/OculusXRInput.OculusXRHandComponent|SetMeshType _bp_oculushand (Variables|Default|GetHand))
  (Variables|/Script/OculusXRInput.OculusXRHandComponent|SetSkeletonType _bp_oculushand (Variables|Default|GetHand)))