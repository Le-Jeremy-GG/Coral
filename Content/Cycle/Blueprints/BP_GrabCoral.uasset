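; Grabbable coral for a VR experience that, once activated, blinks via a material parameter and shows a "Grab the coral" prompt in French or English, per the game instance.
; The first grab clears the cue and, with a valid coral manager, resumes its sequencer, then after a delay clears both pawn hands, detaches and hides the coral.
; The construction script keeps the Scene component upright, preserving only yaw.
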(event Custom|ActivateCoral
  (Variables|Default|SetbCanGrab true)
  (Rendering|Material|SetScalarParameterValueonMaterials (Variables|Default|GetCoralMesh) "SwitchBlink" 1.0)
  (Development|SetHiddeninGame (Variables|Default|Getattraper4_Sprite) false false))

(event Custom|HasGrabbed
  (params (vrpawnref :type VR%20Pawn%20Object%20Reference))
  (Physics|SetSimulatePhysics (Variables|Default|GetCoralMesh) false)
  (Utilities|FlowControl|DoOnce false
    (:Completed
      (bind _coralmanagerref (Variables|Default|GetCoralManagerRef)
        (:then
          (CallFunction|DeactivateBlink)
          (Default|ResumeSequencer _coralmanagerref)
          (Utilities|FlowControl|Delay 19.0)
          (Variables|/Game/VRBase/VRTemplate/Blueprints/VRPawn.VRPawn_C|SetHeldComponentLeft vrpawnref 0)
          (Variables|/Game/VRBase/VRTemplate/Blueprints/VRPawn.VRPawn_C|SetHeldComponentRight vrpawnref 0)
          (Transformation|DetachFromActor "KeepWorld" "KeepWorld" "KeepWorld")
          (Rendering|SetVisibility (Variables|Default|GetCoralMesh) false false)
          (Variables|Default|SetbCanGrab false))
        (:else
          (CallFunction|DeactivateBlink))))))

(event Custom|DeactivateBlink
  (Rendering|Material|SetScalarParameterValueonMaterials (Variables|Default|GetCoralMesh) "SwitchBlink" 0.0)
  (Development|SetHiddeninGame (Variables|Default|Getattraper4_Sprite) true false))

(event EventBeginPlay
  (Rendering|Material|SetScalarParameterValueonMaterials (Variables|Default|GetCoralMesh) "SwitchBlink" 0.0)
  (bind _asgi_cycle (Utilities|Casting|CastToGI_Cycle (Game|GetGameInstance)))
  (Rendering|Components|TextRender|SetText (Variables|Default|GetTextRender) (Utilities|Text|ToText(String) (Utilities|Select :Index (Variables|/Game/Cycle/Blueprints/GI_Cycle.GI_Cycle_C|GetLanguage _asgi_cycle) :NewEnumerator0 "Attrapez 
le corail" :NewEnumerator1 "Grab the 
coral")))
  (Development|SetHiddeninGame (Variables|Default|Getattraper4_Sprite) true false))

(fn ConstructionScript
  (bind _scene (Variables|Default|GetScene))
  (Transformation|SetWorldRotation _scene (Math|Rotator|MakeRotator 0.0 0.0 (.Yaw (Math|Rotator|BreakRotator (Transformation|GetWorldRotation _scene)))) false false))