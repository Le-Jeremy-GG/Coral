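; BP_CoralManager runs the coral scene: it plays the French or English voice sequence chosen in GI_Cycle, then opens Map_Carroussel when it finishes.
; On BeginPlay it registers itself with every BP_GrabCoral, which it can activate together and stop blinking after the first grab.
; Pausing the sequence, only with a headset enabled, shows the VR pawn's hands; resuming hides them after a delay.
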(event Custom|OnFinished
  (Game|OpenLevel(byObjectReference) "/Game/Carroussel/Map_Carroussel.Map_Carroussel"))

(event Custom|HasGrabbedOneCoral
  (Utilities|FlowControl|DoOnce false
    (:Completed
      (for _array_element (Variables|Default|GetCoralGrabList)
        (Default|DeactivateBlink _array_element)))))

(event Custom|EnableGrab
  (for _array_element (Variables|Default|GetCoralGrabList)
    (Default|ActivateCoral _array_element)))

(event Custom|ResumeSequencer
  (Sequencer|Player|Play (Variables|Default|GetSequencerRef) :!class /Script/MovieScene.MovieSceneSequencePlayer)
  (Utilities|FlowControl|Delay 12.0)
  (bind _asvrpawn (Utilities|Casting|CastToVRPawn (Game|Player|GetPlayerPawn 0)))
  (Default|HandVisibility _asvrpawn false))

(event Custom|PauseSequencer
  (if (Class|HeadMountedDisplayFunctionLibrary|IsHeadMountedDisplayEnabled)
    (Sequencer|Player|Pause (Variables|Default|GetSequencerRef))
    (bind _asvrpawn (Utilities|Casting|CastToVRPawn (Game|Player|GetPlayerPawn 0)))
    (Default|HandVisibility _asvrpawn true)))

(event Custom|MakeSomeNoise
  (bind _audio (Variables|Default|GetAudio))
  (Audio|Components|Audio|SetSound _audio (Variables|Default|GetNew%20Sound))
  (Components|Activation|Activate _audio true)
  (Audio|Components|Audio|Play _audio 0.0))

(event EventBeginPlay
  (Utilities|FlowControl|Delay 0.2)
  (Utilities|FlowControl|Sequence
    (:then_0
      (bind _outactors (Actor|GetAllActorsOfClass "/Game/Cycle/Blueprints/BP_GrabCoral.BP_GrabCoral_C"))
      (bind _output_get (Variables|Default|SetCoralGrabList _outactors))
      (for _array_element _output_get
        (Variables|/Game/Cycle/Blueprints/BP_GrabCoral.BP_GrabCoral_C|SetCoralManagerRef _array_element self)))
    (:then_1
      (bind _asgi_cycle (Utilities|Casting|CastToGI_Cycle (Game|GetGameInstance)))
      (switch Utilities|FlowControl|Switch|SwitchonEnum_Language (Variables|/Game/Cycle/Blueprints/GI_Cycle.GI_Cycle_C|GetLanguage _asgi_cycle)
        (:NewEnumerator0
          (bind _returnvalue (Sequencer|Player|CreateLevelSequencePlayer "/Game/Cycle/Sequencer_VoiceFR.Sequencer_VoiceFR"))
          (Variables|Default|SetSequencerRef _returnvalue))
        (:NewEnumerator1
          (bind _returnvalue_2 (Sequencer|Player|CreateLevelSequencePlayer "/Game/Cycle/Sequencer_VoiceEN.Sequencer_VoiceEN"))
          (Variables|Default|SetSequencerRef _returnvalue_2)))
      (Sequencer|Player|Play (Variables|Default|GetSequencerRef) :!class /Script/MovieScene.MovieSceneSequencePlayer)
      (Development|ExecuteConsoleCommand "Sequencer.Audio.UseAudioClockForAudioDesync 1" 0)
      (EventDispatchers|BindEventtoOnFinished (Variables|Default|GetSequencerRef) (delegate Custom|OnFinished)))))

(fn ConstructionScript)