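; Main menu actor that hosts language and main menu widget components and coordinates navigation between them, credits and levels.
; On BeginPlay it links itself to both widgets and finds the credits actor, showing language selection on first launch, otherwise the main menu in the saved language.
; Switch events toggle component visibility and pass the language on, credits swap in with timed fades, and level loads follow a pawn fade to black.
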(event Custom|ShowHideMainMenu
  (params (Hide :type Boolean))
  (Development|SetHiddeninGame (Variables|Default|GetMainMenu) Hide false))

(event Custom|ShowHideLanguageMenu
  (params (Hide :type Boolean))
  (Development|SetHiddeninGame (Variables|Default|GetLanguageMenu) Hide false))

(event Custom|GoToAnimation
  (Default|FadetoBlack (Variables|Default|GetPawnRef))
  (Utilities|Time|SetTimerbyEvent (delegate Custom|OpenMainMap) 1.0))

(event Custom|SwitchToLanguageMenu
  (CallFunction|ShowHideMainMenu true)
  (CallFunction|ShowHideLanguageMenu false)
  (Default|ShowHideLanguage (Variables|Default|GetLanguageMenuRef) true))

(event Custom|SwitchToMainMenu
  (params (LanguageToUse :type Enum_Language%20Enum :default "NewEnumerator0"))
  (bind _output_get (Variables|Default|SetLanguage LanguageToUse))
  (Default|UpdateLanguage (Variables|Default|GetMainMenuRef) _output_get)
  (CallFunction|ShowHideMainMenu false)
  (CallFunction|ShowHideLanguageMenu true)
  (Default|ShowHideMenu (Variables|Default|GetMainMenuRef) true))

(event Custom|GoToCarrousel
  (Default|FadetoBlack (Variables|Default|GetPawnRef))
  (Utilities|Time|SetTimerbyEvent (delegate Custom|OpenCarrouselMap) 1.0))

(event Custom|OpenMainMap
  (Game|OpenLevel(byObjectReference) "/Game/Cycle/M_BlockingMap.M_BlockingMap"))

(event Custom|OpenCarrouselMap
  (Game|OpenLevel(byObjectReference) "/Game/Carroussel/Map_Carroussel.Map_Carroussel"))

(event Custom|MenuToCredits
  (Utilities|FlowControl|Sequence
    (:then_0
      (Utilities|FlowControl|DoOnce false
        (:Completed
          (Default|UpdateText (Variables|Default|GetCredits) (Variables|Default|GetLanguage)))))
    (:then_1
      (Utilities|FlowControl|Delay 0.2)
      (Default|ShowHideMenu (Variables|Default|GetMainMenuRef) false)
      (Utilities|FlowControl|Delay 1.0)
      (CallFunction|ShowHideMainMenu true)
      (Default|Fade (Variables|Default|GetCredits) true))))

(event Custom|CreditsToMenu
  (Default|Fade (Variables|Default|GetCredits) false)
  (Utilities|FlowControl|Delay 1.0)
  (CallFunction|ShowHideMainMenu false)
  (Default|ShowHideMenu (Variables|Default|GetMainMenuRef) true))

(event EventBeginPlay
  (Utilities|FlowControl|Sequence
    (:then_0
      (bind _aswbp_language (Utilities|Casting|CastToWBP_Language (UserInterface|GetWidget (Variables|Default|GetLanguageMenu))))
      (Variables|Default|SetLanguageMenuRef _aswbp_language)
      (Variables|/Game/Cycle/Blueprints/WBP_Language.WBP_Language_C|SetMainMenuRef _aswbp_language self))
    (:then_1
      (bind _aswbp_main_menu (Utilities|Casting|CastToWBP_MainMenu (UserInterface|GetWidget (Variables|Default|GetMainMenu))))
      (Variables|Default|SetMainMenuRef _aswbp_main_menu)
      (Variables|/Game/Cycle/Blueprints/WBP_MainMenu.WBP_MainMenu_C|SetMainMenuBPRef _aswbp_main_menu self))
    (:then_2
      (bind _asgi_cycle (Utilities|Casting|CastToGI_Cycle (Game|GetGameInstance)))
      (if (Variables|/Game/Cycle/Blueprints/GI_Cycle.GI_Cycle_C|GetbIsFirstTime _asgi_cycle)
        (Variables|/Game/Cycle/Blueprints/GI_Cycle.GI_Cycle_C|SetbIsFirstTime _asgi_cycle false)
        (Development|SetHiddeninGame (Variables|Default|GetLanguageMenu) false false)
        (Development|SetHiddeninGame (Variables|Default|GetMainMenu) true false)
        (else
          (bind _output_get (Variables|Default|SetLanguage (Variables|/Game/Cycle/Blueprints/GI_Cycle.GI_Cycle_C|GetLanguage _asgi_cycle)))
          (Default|UpdateLanguage (Variables|Default|GetMainMenuRef) _output_get)
          (Development|SetHiddeninGame (Variables|Default|GetLanguageMenu) true false)
          (Development|SetHiddeninGame (Variables|Default|GetMainMenu) false false)
          (Default|ShowHideMenu (Variables|Default|GetMainMenuRef) true))))
    (:then_3
      (bind _outactors (Actor|GetAllActorsOfClass "/Game/Cycle/MainMenuLogos/A_Credits.A_Credits_C"))
      (Variables|Default|SetCredits (Utilities|Array|Get(acopy) _outactors)))))

(fn ConstructionScript)