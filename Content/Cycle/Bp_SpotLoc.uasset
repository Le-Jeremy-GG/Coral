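; Spot marker actor that publishes its world location to a Material Parameter Collection as SpotPosition, for materials to read.
; Every Tick it pins itself to X = 0, keeping Y and Z, then writes the location to the parameter.
; The construction script writes the same parameter and prints the location as a long-lasting debug string.
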(event EventBeginPlay)

(event Collision|EventActorBeginOverlap
  (params (OtherActor :type Actor%20Object%20Reference)))

(event EventTick
  (params (DeltaSeconds :type Float%20%28single-precision%29))
  (bind _returnvalue (Transformation|GetActorLocation))
  (bind _returnvalue_2 (Transformation|GetActorLocation))
  (Transformation|SetActorLocation (Math|Vector|MakeVector 0.0 (.y _returnvalue) (.z _returnvalue)) false false)
  (Rendering|Material|SetVectorParameterValue "/Game/Common/materials/MPC.MPC" "SpotPosition" (Math|Color|MakeColor (.x _returnvalue_2) (.y _returnvalue_2) (.z _returnvalue_2)) :!class /Script/Engine.KismetMaterialLibrary))

(fn ConstructionScript
  (bind _returnvalue (Transformation|GetActorLocation))
  (Rendering|Material|SetVectorParameterValue "/Game/Common/materials/MPC.MPC" "SpotPosition" (Math|Color|MakeColor (.x _returnvalue) (.y _returnvalue) (.z _returnvalue)) :!class /Script/Engine.KismetMaterialLibrary)
  (Development|PrintString (Utilities|String|ToString(Integer) (Math|Conversions|ToLinearColor(Vector) (Transformation|GetActorLocation))) true true "(R=0.000000,G=0.660000,B=1.000000,A=1.000000)" 2e+02))